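; Player controller for the NDI examples that broadcasts the active viewport and lets the player switch broadcasting on and off.
; BeginPlay adds the WB_ViewportBroadcastHUD widget to the screen, then starts broadcasting and stores the result in a state flag.
; Insert starts and Delete stops the broadcast, each guarded by that flag and firing the broadcast-mode-changed event, which BeginPlay does not fire.
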(event EventBeginPlay
  ;[0.5 0 0] Begin Play:
  ; (1) Cretae HUD Widget
  ; (2) begin Broadcasting Acctive Viewport
  (Utilities|FlowControl|Sequence
    (:then_0
      ;;[0 0 0] Create Widget for this Controller
      (bind _returnvalue (UserInterface|CreateWidget "/Game/NDIExamplesContent/Blueprints/Widgets/ViewportBroadcast/WB_ViewportBroadcastHUD.WB_ViewportBroadcastHUD_C" self))
      (UserInterface|Viewport|AddtoViewport _returnvalue 0))
    (:then_1
      ;;[0 0 0] Begin Broadcasting Active Viewport
      (bind _returnvalue_2 (Class|NDIIOLibrary|BeginBroadcastingActiveViewport))
      (Variables|Default|SetIs%20Currently%20Broadcasting%20Active%20Viewport? _returnvalue_2))))

(event Input|KeyboardEvents|Insert
  (params (Key :type Key%20Structure))
  ;[0 0.2 0.5] Insert Key Handler: Begin Broadcasting Active Viewport
  (:Pressed
    (if (not (Variables|Default|GetIs%20Currently%20Broadcasting%20Active%20Viewport?))
      (bind _returnvalue (Class|NDIIOLibrary|BeginBroadcastingActiveViewport))
      (bind _output_get (Variables|Default|SetIs%20Currently%20Broadcasting%20Active%20Viewport? _returnvalue))
      (Default|CallOnBroadcastModeChangedEvent _output_get))))

(event Input|KeyboardEvents|Delete
  (params (Key :type Key%20Structure))
  ;[0 0.2 0.5] Delete Key Handler: Stop Broadcasting Active Viewport
  (:Pressed
    (if (Variables|Default|GetIs%20Currently%20Broadcasting%20Active%20Viewport?)
      (Class|NDIIOLibrary|StopBroadcastingActiveViewport)
      (bind _output_get (Variables|Default|SetIs%20Currently%20Broadcasting%20Active%20Viewport? false))
      (Default|CallOnBroadcastModeChangedEvent _output_get))))

(fn ConstructionScript)