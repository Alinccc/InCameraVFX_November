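; Player controller for an NDI example that automatically connects to a named network video stream.
; On BeginPlay it adds the simple input HUD and searches the NDI Finder component for the configured stream name, retrying whenever network sources change.
; Once found, it starts the NDI Receiver on that connection and notifies listeners through a dispatcher.
; A receiving flag blocks further searches and is never cleared here.
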(event OnNetworkSourcesChanged(NDIFinderComponent)
  (params (InComponent :type NDI%20Finder%20Component%20Object%20Reference))
  ;[0.25 0 0] Event: On Network Sources Changed
  (CallFunction|EventonFindNetworkConnectionandStream))

(event Custom|Event%20On%20Find%20Network%20Connection%20and%20Stream
  ;[0 0.25 1] Event: On Find Network Connection and Stream
  ; (1)  Check if we are currently streaming
  ; (2) Using the 'Stream Name' property 'Find Network Source by Name' and set the connection
  ; (3) If the Source Name was found on the network, Start Receving the stream and Trigger the Dispatcher Notifying any Listeners
  (if (not (Variables|Default|GetIs%20Currently%20Receiving%20Stream?))
    (bind (_connectioninformation _returnvalue) (Class|NDIFinderComponent|FindNetworkSourcebyName (Variables|Default|GetNDI%20Finder%20Component) (Variables|Default|GetStream%20Name)))
    (Variables|Default|SetCurrent%20Connection _connectioninformation)
    (if _returnvalue
      (Variables|Default|SetIs%20Currently%20Receiving%20Stream? true)
      (Class|NDIReceiverComponent|StartReceiver (Variables|Default|GetNDI%20Receiver%20Component) (Variables|Default|GetCurrent%20Connection))
      (Class|NDIReceiverComponent|ChangeConnection (Variables|Default|GetNDI%20Receiver%20Component) (Variables|Default|GetCurrent%20Connection))
      (Default|CallChangeNetworkSourceConnection (Utilities|Text|ToText(String) (.SourceName (Utilities|Struct|BreakNDIConnectionInformation (Variables|Default|GetCurrent%20Connection))))))))

(event EventBeginPlay
  ;[0.25 0 0] Begin Play:
  ; (1) Create HUD Widget to display on screen
  ; (2) Call Find Network Connection and Stream
  (bind _returnvalue (UserInterface|CreateWidget "/Game/NDIExamplesContent/Blueprints/Widgets/SimpleInput/WB_SimpleInputHUD.WB_SimpleInputHUD_C" self))
  (UserInterface|Viewport|AddtoViewport _returnvalue 0)
  (CallFunction|EventonFindNetworkConnectionandStream))

(fn ConstructionScript)