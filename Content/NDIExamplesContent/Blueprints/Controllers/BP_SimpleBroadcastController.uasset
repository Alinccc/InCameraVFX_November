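; Player controller for an NDI example that toggles broadcasting through its NDIBroadcastComponent.
; On BeginPlay it adds the broadcast HUD to the viewport, starts broadcasting at once, then announces the resulting state after a short delay.
; Insert starts and Delete stops the broadcast, guarded by IsCurrentlyBroadcasting and component validity.
; Each change is reported through CallOnBroadcastingModeChangedEvent.
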(event EventBeginPlay
  (Utilities|FlowControl|Sequence
    (:then_0
      (bind _returnvalue (UserInterface|CreateWidget "/Game/NDIExamplesContent/Blueprints/Widgets/SimpleBroadcast/WB_SimpleBroadcastHUD.WB_SimpleBroadcastHUD_C" self))
      (UserInterface|Viewport|AddtoViewport _returnvalue 0))
    (:then_1
      (bind _returnvalue_2 (Class|NDIBroadcastComponent|StartBroadcasting (Variables|Default|GetNDI%20Broadcast%20Component)))
      (Variables|Default|SetIs%20Currently%20Broadcasting? _returnvalue_2)
      (Utilities|FlowControl|Delay 1.5)
      (Default|CallOnBroadcastingModeChangedEvent (Variables|Default|GetIs%20Currently%20Broadcasting?)))))

(event Input|KeyboardEvents|Insert
  (params (Key :type Key%20Structure))
  (:Pressed
    (if (not (Variables|Default|GetIs%20Currently%20Broadcasting?))
      (bind _ndi_broadcast_component (Variables|Default|GetNDI%20Broadcast%20Component)
        (:then
          (bind _returnvalue (Class|NDIBroadcastComponent|StartBroadcasting _ndi_broadcast_component))
          (bind _output_get (Variables|Default|SetIs%20Currently%20Broadcasting? _returnvalue))
          (Default|CallOnBroadcastingModeChangedEvent _output_get))
        (:else)))))

(event Input|KeyboardEvents|Delete
  (params (Key :type Key%20Structure))
  (:Pressed
    (if (Variables|Default|GetIs%20Currently%20Broadcasting?)
      (bind _ndi_broadcast_component (Variables|Default|GetNDI%20Broadcast%20Component)
        (:then
          (Class|NDIBroadcastComponent|StopBroadcasting _ndi_broadcast_component)
          (bind _output_get (Variables|Default|SetIs%20Currently%20Broadcasting? false))
          (Default|CallOnBroadcastingModeChangedEvent _output_get))
        (:else)))))

(fn ConstructionScript)